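; Player controller for a map-based army game that handles camera panning, army selection and move orders.
; MoveUnit traces under the cursor, selecting all friendly army pawns sharing the clicked Id, or sending the selection via AIMoveTo toward an enemy or point.
; The selection clears after each order.
; Tick moves the camera pawn along normalized axis input, clamped to map size measured from BP_MapGrid bounds shortly after BeginPlay.
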(event EventBeginPlay
  ;[1 1 1] Find out Map Size / Set Camera Pawn
  (Variables|Default|SetbShowMouseCursor true)
  (Variables|Default|SetCameraPawn (Game|Player|GetPlayerPawn 0))
  (Utilities|FlowControl|Delay 0.2)
  (bind _returnvalue (Actor|GetActorOfClass "/Game/Blueprints/BP_MapGrid.BP_MapGrid_C"))
  (Variables|Default|SetMapXSize (* (.X (Math|Vector|BreakVector (.BoxExtent (Collision|GetActorBounds _returnvalue false false)))) 2.0))
  (Variables|Default|SetMapYSize (* (.Y (Math|Vector|BreakVector (.BoxExtent (Collision|GetActorBounds _returnvalue false false)))) 2.0)))

(event EventTick
  (params (DeltaSeconds :type Float%20%28single-precision%29))
  (bind _cameraspeed (Variables|Default|GetCameraSpeed))
  (bind _camerapawn (Variables|Default|GetCameraPawn))
  (bind _cameramovment (Variables|Default|GetCameraMovment))
  (bind _returnvalue (Math|Vector|Normalize _cameramovment))
  (bind _returnvalue_2 (Transformation|GetActorLocation _camerapawn))
  (bind _returnvalue_3 (* _returnvalue _cameraspeed))
  (bind _returnvalue_4 (+ _returnvalue_2 _returnvalue_3))
  (bind (_x _y _z) (Math|Vector|BreakVector _returnvalue_4))
  ;[1 1 1] Move Camera
  (Transformation|SetActorLocation _camerapawn (Math|Vector|MakeVector (Math|Float|Clamp(Float) _x 0.0 (Variables|Default|GetMapXSize)) (Math|Float|Clamp(Float) _y 0.0 (Variables|Default|GetMapYSize)) _z) false false))

(event Input|ActionEvents|InputActionMoveUnit
  (params (Key :type Key%20Structure :default "None"))
  (bind _hitresult (Game|Player|GetHitResultUnderCursorbyChannel "TraceTypeQuery1" true))
  (bind _armypawn (Variables|Default|GetArmyPawn))
  (bind (_bblockinghit _binitialoverlap _time _distance _location _impactpoint _normal _impactnormal _physmat _hitactor) (Collision|BreakHitResult _hitresult))
  (:Pressed
    (bind _asbp_army_pawn (Utilities|Casting|CastToBP_ArmyPawn _hitactor)
      (:then
        (if (Variables|/Game/Blueprints/BP_ArmyPawn.BP_ArmyPawn_C|GetIsEnemy _asbp_army_pawn)
          ;[1 1 1] Send Movment Command to Army Pawn
          (for _array_element _armypawn
            (AI|AIMoveTo _array_element "0, 0, 0" _asbp_army_pawn 1e+01 true))
          (Utilities|Array|Clear (Variables|Default|GetArmyPawn) :!label _label)
          (Rendering|Debug|DrawDebugSphere _location 5.0 12 "(R=1.000000,G=1.000000,B=1.000000,A=1.000000)" 0.0)
          (else
            ;[1 1 1] Select Army
            (Utilities|Array|Clear (Variables|Default|GetArmyPawn))
            (bind _outactors (Actor|GetAllActorsOfClass "/Game/Blueprints/BP_ArmyPawn.BP_ArmyPawn_C"))
            (for _array_element_2 _outactors
              (if (== (Variables|/Game/Blueprints/BP_ArmyPawn.BP_ArmyPawn_C|GetId _array_element_2) (Variables|/Game/Blueprints/BP_ArmyPawn.BP_ArmyPawn_C|GetId _asbp_army_pawn))
                (Utilities|Array|Add (Variables|Default|GetArmyPawn) _array_element_2)
                (Audio|PlaySound2D "/Game/Sound/select.select" 1.0 1.0 0.0 0 0))))))
      (:CastFailed
        (for _array_element_3 _armypawn
          (AI|AIMoveTo _array_element_3 _location 0 1e+01 true))
        (goto _label)))))

(event Input|AxisEvents|InputAxisAxisNorthSouth
  (params (AxisValue :type Float%20%28single-precision%29))
  ;[1 1 1] Receive Camera Movment
  (Variables|Default|SetCameraMovment (Math|Vector|MakeVector AxisValue (.Y (Math|Vector|BreakVector (Variables|Default|GetCameraMovment))) (.Z (Math|Vector|BreakVector (Variables|Default|GetCameraMovment))))))

(event Input|AxisEvents|InputAxisAxisEastWest
  (params (AxisValue :type Float%20%28single-precision%29))
  ;[1 1 1] Receive Camera Movment
  (Variables|Default|SetCameraMovment (Math|Vector|MakeVector (.X (Math|Vector|BreakVector (Variables|Default|GetCameraMovment))) AxisValue (.Z (Math|Vector|BreakVector (Variables|Default|GetCameraMovment))))))

(fn ConstructionScript)