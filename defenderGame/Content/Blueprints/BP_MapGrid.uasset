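; BP_MapGrid is a tile map actor that builds a grid level from the TileMap array in its construction script.
; Nested Height and Width loops read the flattened array and place each tile at TileSize spacing, with rows along local X.
; Tile values select default, forest or river instanced mesh components, with unknown values falling back to default.
; Forest tiles also get their own box component at the same location.
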(event EventBeginPlay)

(event Collision|EventActorBeginOverlap
  (params (OtherActor :type Actor%20Object%20Reference)))

(event EventTick
  (params (DeltaSeconds :type Float%20%28single-precision%29)))

(fn ConstructionScript
  (bind _width (Variables|Default|GetWidth))
  (bind _tilesize (Variables|Default|GetTileSize))
  ;[1 1 1] Create Map
  (for _index (range 0 (+ (Variables|Default|GetHeight) -1))
    (for _index_2 (range 0 (+ _width -1))
      (switch int (Utilities|Array|Get(acopy) (Variables|Default|GetTileMap) (+ _index_2 (* _index _width)))
        (:Default
          (Components|InstancedStaticMesh|AddInstance (Variables|Default|GetDefaultTiles) (Math|Transform|MakeTransform (Math|Vector|MakeVector (* (Math|Conversions|ToFloat(Integer) _index) _tilesize) (* (Math|Conversions|ToFloat(Integer) _index_2) _tilesize) 0.0)) false :!label _label))
        (:0
          (goto _label))
        (:1
          (Components|InstancedStaticMesh|AddInstance (Variables|Default|GetForrestTiles) (Math|Transform|MakeTransform (Math|Vector|MakeVector (* (Math|Conversions|ToFloat(Integer) _index) _tilesize) (* (Math|Conversions|ToFloat(Integer) _index_2) _tilesize) 0.0)) false)
          (AddComponent|AddBoxComponent false (Math|Transform|MakeTransform (Math|Vector|MakeVector (* (Math|Conversions|ToFloat(Integer) _index) _tilesize) (* (Math|Conversions|ToFloat(Integer) _index_2) _tilesize) 0.0))))
        (:2
          (Components|InstancedStaticMesh|AddInstance (Variables|Default|GetRiverTiles) (Math|Transform|MakeTransform (Math|Vector|MakeVector (* (Math|Conversions|ToFloat(Integer) _index) _tilesize) (* (Math|Conversions|ToFloat(Integer) _index_2) _tilesize) 0.0)) false))))))