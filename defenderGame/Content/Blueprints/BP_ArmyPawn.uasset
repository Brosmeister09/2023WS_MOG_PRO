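; BP_ArmyPawn is a base army unit pawn that moves by AI and tracks opponents for combat.
; Its CombatDetector adds and removes opposite-side BP_HealthObjects tagged army or castle, setting IsInCombat while any remain.
; Box overlaps halve and restore movement speed when the event's OverlappedComponent has the slow tag.
; Move events wrap AIMoveTo for actors or locations, and the empty Attack function is left for child classes to override.
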(event OnComponentBeginOverlap(CombatDetector)
  (params (OverlappedComponent :type Primitive%20Component%20Object%20Reference) (OtherActor :type Actor%20Object%20Reference) (OtherComp :type Primitive%20Component%20Object%20Reference) (OtherBodyIndex :type Integer) (bFromSweep :type Boolean) (SweepResult :type Hit%20Result%20Structure%20%28by%20ref%29))
  (bind _opponents (Variables|Default|GetOpponents))
  (if (or (Components|ComponentHasTag OtherComp "army") (Components|ComponentHasTag OtherComp "castle"))
    (bind _asbp_health_object (Utilities|Casting|CastToBP_HealthObject OtherActor))
    (if (Class|KismetMathLibrary|XORBoolean (Variables|/Game/Blueprints/BP_HealthObject.BP_HealthObject_C|GetIsEnemy _asbp_health_object) (Variables|Default|GetIsEnemy))
      (Utilities|Array|Add _opponents _asbp_health_object)
      (if (>= (Utilities|Array|Length _opponents) 1)
        (Variables|Default|SetIsInCombat true)))))

(event OnComponentEndOverlap(CombatDetector)
  (params (OverlappedComponent :type Primitive%20Component%20Object%20Reference) (OtherActor :type Actor%20Object%20Reference) (OtherComp :type Primitive%20Component%20Object%20Reference) (OtherBodyIndex :type Integer))
  (bind _opponents (Variables|Default|GetOpponents))
  (if (or (Components|ComponentHasTag OtherComp "army") (Components|ComponentHasTag OtherComp "castle"))
    (bind _asbp_health_object (Utilities|Casting|CastToBP_HealthObject OtherActor))
    (if (Class|KismetMathLibrary|XORBoolean (Variables|/Game/Blueprints/BP_HealthObject.BP_HealthObject_C|GetIsEnemy _asbp_health_object) (Variables|Default|GetIsEnemy))
      (Utilities|Array|RemoveItem _opponents _asbp_health_object)
      (if (< (Utilities|Array|Length _opponents) 1)
        (Variables|Default|SetIsInCombat false)))))

(event OnComponentBeginOverlap(Box)
  (params (OverlappedComponent :type Primitive%20Component%20Object%20Reference) (OtherActor :type Actor%20Object%20Reference) (OtherComp :type Primitive%20Component%20Object%20Reference) (OtherBodyIndex :type Integer) (bFromSweep :type Boolean) (SweepResult :type Hit%20Result%20Structure%20%28by%20ref%29))
  (bind _floatingpawnmovement (Variables|Default|GetFloatingPawnMovement))
  (if (Utilities|IsValid OverlappedComponent)
    (if (Components|ComponentHasTag OverlappedComponent "slow")
      (Variables|/Script/Engine.FloatingPawnMovement|SetMaxSpeed _floatingpawnmovement (/ (Class|MovementComponent|GetMaxSpeed _floatingpawnmovement) 2.0)))))

(event OnComponentEndOverlap(Box)
  (params (OverlappedComponent :type Primitive%20Component%20Object%20Reference) (OtherActor :type Actor%20Object%20Reference) (OtherComp :type Primitive%20Component%20Object%20Reference) (OtherBodyIndex :type Integer))
  (bind _floatingpawnmovement (Variables|Default|GetFloatingPawnMovement))
  (if (Utilities|IsValid OverlappedComponent)
    (if (Components|ComponentHasTag OverlappedComponent "slow")
      (Variables|/Script/Engine.FloatingPawnMovement|SetMaxSpeed _floatingpawnmovement (* (Class|MovementComponent|GetMaxSpeed _floatingpawnmovement) 2.0)))))

(event Custom|MoveToLocation
  (params (TargetLocation :type Vector))
  (AI|AIMoveTo self TargetLocation 0 1e+01 false))

(event Custom|MoveToActor
  (params (TargetActor :type Actor%20Object%20Reference))
  (Utilities|IsValid TargetActor
    (:Is%20Valid
      (AI|AIMoveTo self "0, 0, 0" TargetActor 1e+01 false))))

(fn ConstructionScript)

(fn Attack
  ;[1 1 1] This function is ment to be overwritten by the children of this class so they can have their own unique attack behaviour
)