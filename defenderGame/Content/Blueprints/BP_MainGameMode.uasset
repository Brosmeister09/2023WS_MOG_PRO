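; Game mode for a castle game that moves the player pawn over the map grid at start, manages money and army spawning, and triggers game over once no castle exists.
; SpawnUnit places three units sharing an Id in a row beside the castle, destroying that group if any spawn fails.
; Only successful spawns deduct the cost.
; AddMoney grants a fixed income, and both money changes update the HUD.
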(event Custom|Add%20Money
  (bind _output_get (Variables|Default|SetMoney (+ (Variables|Default|GetMoney) 15)))
  (bind _asmain_hud (Utilities|Casting|CastTomainHUD (HUD|GetHUD (Game|GetPlayerController 0))))
  (Default|UpdateMoney (Variables|/Game/UI/mainHUD.mainHUD_C|GetUIRef _asmain_hud) _output_get))

(event EventBeginPlay
  ;[1 1 1] Center Camera at the Center of Map
  (Utilities|FlowControl|Delay 0.5)
  (bind _returnvalue (Actor|GetActorOfClass "/Game/Blueprints/BP_MapGrid.BP_MapGrid_C"))
  (Transformation|SetActorLocationAndRotation (Game|Player|GetPlayerPawn 0) (.BoxExtent (Collision|GetActorBounds _returnvalue false false))))

(event EventTick
  (params (DeltaSeconds :type Float%20%28single-precision%29))
  (bind _returnvalue (Actor|GetActorOfClass "/Game/Blueprints/BP_Castle.BP_Castle_C"))
  (if (not (Utilities|IsValid _returnvalue))
    (bind _asmain_hud (Utilities|Casting|CastTomainHUD (HUD|GetHUD (Game|GetPlayerController 0))))
    (Default|GameOver _asmain_hud)))

(fn ConstructionScript)

(fn GetSpawnPostionBeforeCastle
  (params (A :type Integer))
  (bind _returnvalue (Actor|GetActorOfClass "/Game/Blueprints/BP_Castle.BP_Castle_C"))
  (return (Math|Transform|MakeTransform (Math|Vector|MakeVector (.X (Math|Vector|BreakVector (- (.Origin (Collision|GetActorBounds _returnvalue false false)) (Math|Vector|MakeVector (+ (.X (Math|Vector|BreakVector (.BoxExtent (Collision|GetActorBounds _returnvalue false false)))) 2e+01) 0.0 0.0)))) (+ (.Y (Math|Vector|BreakVector (- (.Origin (Collision|GetActorBounds _returnvalue false false)) (Math|Vector|MakeVector (+ (.X (Math|Vector|BreakVector (.BoxExtent (Collision|GetActorBounds _returnvalue false false)))) 2e+01) 0.0 0.0)))) (* A 30)) 1e+01) "0.000000,180.000000,0.000000")))

(fn SpawnUnit
  (params (BP_Army_Class :type BP%20Army%20Pawn%20Class%20Reference) (Cost :type Integer))
  ;[1 1 1] Spawn Unit
  (if (>= (Variables|Default|GetMoney) Cost)
    (Variables|Default|SetBP_Army_Class BP_Army_Class)
    (Variables|Default|Setlast_id (+ (Variables|Default|Getlast_id) 1))
    (bind _index (Utilities|FlowControl|ForLoopwithBreak -1 1 :!label _label)
      (:LoopBody
        (bind _returnvalue (CallFunction|GetSpawnPostionBeforeCastle _index))
        (bind _returnvalue_2 (Game|SpawnActorfromClass (Variables|Default|GetBP_Army_Class) _returnvalue "AdjustIfPossibleButDontSpawnIfColliding" "MultiplyWithRoot" 0 (Variables|Default|Getlast_id) 0))
        ;;[1 1 1] Check if Army can be Spawned if not destroy it
        (if (not (Utilities|IsValid _returnvalue_2))
          (bind _outactors (Actor|GetAllActorsOfClass "/Game/Blueprints/BP_ArmyPawn.BP_ArmyPawn_C"))
          (for _array_element _outactors
            (if (== (Variables|/Game/Blueprints/BP_ArmyPawn.BP_ArmyPawn_C|GetId _array_element) (Variables|Default|Getlast_id))
              (Actor|DestroyActor _array_element)))
          (goto _label Break)))
      (:Completed
        (if (Utilities|IsValid _returnvalue_2)
          (Audio|PlaySound2D "/Game/Sound/spawn.spawn" 1.0 1.0 0.0 0 0)
          (bind _output_get (Variables|Default|SetMoney (- (Variables|Default|GetMoney) Cost)))
          (bind _asmain_hud (Utilities|Casting|CastTomainHUD (HUD|GetHUD (Game|GetPlayerController 0))))
          (Default|UpdateMoney (Variables|/Game/UI/mainHUD.mainHUD_C|GetUIRef _asmain_hud) _output_get)
          (else
            (Development|PrintString "Army couldnt be spawned" :!label _label_2)))))
    (else
      (goto _label_2))))