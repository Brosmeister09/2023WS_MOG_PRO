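; BP_SwordFighter is a fighter Blueprint that overrides an inherited Attack to provide an AI-driven melee sword attack.
; After the parent call, Attack validates a random Opponents entry, issues an AI move toward one, subtracts one Health and plays a 2D sword sound.
; The random index re-evaluates at each use, so the checked, approached and damaged opponents can differ.
; Damage lands immediately, without waiting for the move to finish.
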(event EventBeginPlay
  (|CallParentFunction) ; This node is disabled and will not be called.\nDrag off pins to build functionality.
)

(event Collision|EventActorBeginOverlap
  (params (OtherActor :type Actor%20Object%20Reference))
  (|CallParentFunction OtherActor) ; This node is disabled and will not be called.\nDrag off pins to build functionality.
)

(event EventTick
  (params (DeltaSeconds :type Float%20%28single-precision%29))
  (|CallParentFunction DeltaSeconds) ; This node is disabled and will not be called.\nDrag off pins to build functionality.
)

(fn ConstructionScript
  (|CallParentFunction))

(fn Attack
  (bind _opponents (Variables|Default|GetOpponents))
  (bind _returnvalue (Utilities|Array|Length _opponents))
  (bind _returnvalue_2 (- _returnvalue 1))
  (bind _returnvalue_3 (Math|Random|RandomIntegerinRange 0 _returnvalue_2))
  (bind _output (Utilities|Array|Get(acopy) _opponents _returnvalue_3))
  (|CallParentFunction)
  (if (Utilities|IsValid _output)
    (AI|Navigation|MovetoActor (AI|GetAIController self) _output 1.0 true true true 0)
    (Variables|/Game/Blueprints/BP_HealthObject.BP_HealthObject_C|SetHealth _output (- (Variables|/Game/Blueprints/BP_HealthObject.BP_HealthObject_C|GetHealth _output) 1))
    (Audio|PlaySound2D "/Game/Sound/sword_hit.sword_hit" 1.0 1.0 0.0 0 0)))