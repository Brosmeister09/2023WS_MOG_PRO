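; BP_Arrow is an arrow projectile that flies in an arc at a target army and damages what it hits.
; On BeginPlay it computes a launch velocity toward TargetArmy's current location with SuggestProjectileVelocityCustomArc and sets its ProjectileMovement to rotate with velocity.
; When its Box overlaps a component tagged "army" on a BP_HealthObject, it subtracts a fixed amount of Health and destroys itself.
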(event OnComponentBeginOverlap(Box)
  (params (OverlappedComponent :type Primitive%20Component%20Object%20Reference) (OtherActor :type Actor%20Object%20Reference) (OtherComp :type Primitive%20Component%20Object%20Reference) (OtherBodyIndex :type Integer) (bFromSweep :type Boolean) (SweepResult :type Hit%20Result%20Structure%20%28by%20ref%29))
  (if (Components|ComponentHasTag OtherComp "army")
    (bind _asbp_health_object (Utilities|Casting|CastToBP_HealthObject OtherActor))
    (Variables|/Game/Blueprints/BP_HealthObject.BP_HealthObject_C|SetHealth _asbp_health_object (- (Variables|/Game/Blueprints/BP_HealthObject.BP_HealthObject_C|GetHealth _asbp_health_object) 1.5))
    (Actor|DestroyActor)))

(event EventBeginPlay
  (bind _projectilemovement (Variables|Default|GetProjectileMovement))
  (bind _outlaunchvelocity (Game|SuggestProjectileVelocityCustomArc (Transformation|GetActorLocation) (Transformation|GetActorLocation (Variables|Default|GetTargetArmy)) 0.0 0.5))
  (Variables|/Script/Engine.MovementComponent|SetVelocity _projectilemovement _outlaunchvelocity)
  (Variables|/Script/Engine.ProjectileMovementComponent|SetbRotationFollowsVelocity _projectilemovement true))

(fn ConstructionScript)