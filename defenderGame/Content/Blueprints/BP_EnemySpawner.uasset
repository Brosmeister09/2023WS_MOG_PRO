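; BP_EnemySpawner is an actor that periodically spawns BP_EnemyFighter enemies around its own location.
; On BeginPlay it starts a looping timer at the EnemySpawnTime interval, with some variance on the initial delay, that calls SpawnEnemy by function name.
; SpawnEnemy offsets the actor's location randomly in X and Y within SpawnRadius, giving a square area at the same height with zero rotation.
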(event EventBeginPlay
  (Utilities|Time|SetTimerbyFunctionName 0 "SpawnEnemy" (Variables|Default|GetEnemySpawnTime) true 0.0 1.0))

(event Collision|EventActorBeginOverlap
  (params (OtherActor :type Actor%20Object%20Reference)))

(event EventTick
  (params (DeltaSeconds :type Float%20%28single-precision%29)))

(fn ConstructionScript)

(fn SpawnEnemy
  (bind _spawnradius (Variables|Default|GetSpawnRadius))
  (bind _returnvalue (* _spawnradius -1.0))
  (Game|SpawnActorfromClass "/Game/Blueprints/BP_EnemyFighter.BP_EnemyFighter_C" (Math|Transform|MakeTransform (+ (Transformation|GetActorLocation) (Math|Vector|MakeVector (Math|Random|RandomFloatinRange _returnvalue _spawnradius) (Math|Random|RandomFloatinRange _returnvalue _spawnradius) 0.0))) "Undefined" "MultiplyWithRoot" 0 -1 0))