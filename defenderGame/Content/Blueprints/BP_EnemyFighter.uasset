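; BP_EnemyFighter is a melee enemy that marches on the castle and damages opponents, extending inherited parent behavior.
; On BeginPlay, and every Tick while out of combat, it looks up BP_Castle and moves toward it.
; Attack moves to an opponent, subtracts one Health and plays a sword sound; the random pick is re-evaluated at each use, so these steps can hit different opponents.
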(event EventBeginPlay
  (bind _self self)
  (|CallParentFunction)
  (bind _returnvalue (Actor|GetActorOfClass "/Game/Blueprints/BP_Castle.BP_Castle_C"))
  (Utilities|IsValid _returnvalue
    (:Is%20Valid
      (Utilities|IsValid _self
        (:Is%20Valid
          (Default|MovetoActor _self _returnvalue))))))

(event EventTick
  (params (DeltaSeconds :type Float%20%28single-precision%29))
  (bind _self self)
  (|CallParentFunction DeltaSeconds)
  (if (not (Variables|Default|GetIsInCombat))
    (bind _returnvalue (Actor|GetActorOfClass "/Game/Blueprints/BP_Castle.BP_Castle_C"))
    (Utilities|IsValid _returnvalue
      (:Is%20Valid
        (Utilities|IsValid _self
          (:Is%20Valid
            (Default|MovetoActor _self _returnvalue)))))))

(fn ConstructionScript
  (|CallParentFunction))

(fn Attack
  (bind _opponents (Variables|Default|GetOpponents))
  (bind _returnvalue (Utilities|Array|Length _opponents))
  (bind _returnvalue_2 (- _returnvalue 1))
  (bind _returnvalue_3 (Math|Random|RandomIntegerinRange 0 _returnvalue_2))
  (bind _output (Utilities|Array|Get(acopy) _opponents _returnvalue_3))
  (|CallParentFunction)
  (Utilities|IsValid _output
    (:Is%20Valid
      (Default|MovetoActor self _output)
      (Variables|/Game/Blueprints/BP_HealthObject.BP_HealthObject_C|SetHealth _output (- (Variables|/Game/Blueprints/BP_HealthObject.BP_HealthObject_C|GetHealth _output) 1))
      (Audio|PlaySound2D "/Game/Sound/sword_hit.sword_hit" 1.0 1.0 0.0 0 0))))