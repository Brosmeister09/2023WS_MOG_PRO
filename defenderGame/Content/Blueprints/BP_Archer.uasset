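; BP_Archer is an archer unit Blueprint that extends its parent's Attack to shoot arrows at random opponents.
; After the parent call, it validates a random Opponents entry, turns to face one, and spawns a BP_Arrow slightly above itself, passing an opponent as TargetArmy.
; The random pick is an uncached pure node, so the validated, faced and targeted opponents can differ.
; The event graph holds only disabled default events.
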(event EventBeginPlay
  (|CallParentFunction) ; This node is disabled and will not be called.\nDrag off pins to build functionality.
)

(event Collision|EventActorBeginOverlap
  (params (OtherActor :type Actor%20Object%20Reference))
  (|CallParentFunction OtherActor) ; This node is disabled and will not be called.\nDrag off pins to build functionality.
)

(event EventTick
  (params (DeltaSeconds :type Float%20%28single-precision%29))
  (|CallParentFunction DeltaSeconds) ; This node is disabled and will not be called.\nDrag off pins to build functionality.
)

(fn ConstructionScript
  (|CallParentFunction))

(fn Attack
  (bind _returnvalue (Transformation|GetActorLocation))
  (bind _opponents (Variables|Default|GetOpponents))
  (bind _returnvalue_2 (Utilities|Array|Length _opponents))
  (bind (_x _y _z) (Math|Vector|BreakVector _returnvalue))
  (bind _returnvalue_3 (- _returnvalue_2 1))
  (bind _returnvalue_4 (Math|Random|RandomIntegerinRange 0 _returnvalue_3))
  (bind _output (Utilities|Array|Get(acopy) _opponents _returnvalue_4))
  (bind _returnvalue_5 (Transformation|GetActorLocation _output))
  (bind _returnvalue_6 (Math|Rotator|FindLookatRotation _returnvalue _returnvalue_5))
  (|CallParentFunction)
  (if (Utilities|IsValid _output)
    (Transformation|SetActorRotation _returnvalue_6)
    (Game|SpawnActorfromClass "/Game/Blueprints/BP_Arrow.BP_Arrow_C" (Math|Transform|MakeTransform (Math|Vector|MakeVector _x _y (+ _z 3e+01)) _returnvalue_6) "Undefined" "MultiplyWithRoot" 0 _output 0)))